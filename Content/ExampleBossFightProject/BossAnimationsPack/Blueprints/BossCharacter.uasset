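; Boss enemy character that shows a HUD widget, turns to face the player every tick until death, and exposes a damage-window flag.
; Damage, gated by a short DoOnce cooldown, reduces health, shakes the camera and triggers an impulse-driven physical hit reaction.
; A timeline drives the physics blend weight, applied each tick with a physical animation profile.
; At zero health it stops AI logic, sets the death animation, removes the widget and destroys itself.
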(event Custom|DoDamage
  ;[1 1 1] Do/Don't damage
  (Variables|Default|SetIs_Damage_Time true))

(event Custom|DontDamage
  ;[1 1 1] Do/Don't damage
  (Variables|Default|SetIs_Damage_Time false))

(event Custom|PhysicalHitReact
  ;[1 1 1] Physical animation
  (Class|SkeletalMeshComponent|SetAllBodiesBelowPhysicsBlendWeight (Variables|Character|GetMesh) (Variables|Default|GetBoneName) (Variables|Default|GetPhysics%20Blend%20Weight) false false)
  (Class|PhysicalAnimationComponent|ApplyPhysicalAnimationProfileBelow (Variables|Default|GetPhysicalAnimation) (Variables|Default|GetBoneName) "DamagePhysics" true false))

(event EventBeginPlay
  (bind _mesh (Variables|Character|GetMesh))
  ;[1 1 1] Create Widget
  (bind _returnvalue (UserInterface|CreateWidget "/Game/ExampleBossFightProject/BossAnimationsPack/Widget/BossWidget.BossWidget_C" (Game|GetPlayerController 0)))
  (Variables|Default|SetBossWidget _returnvalue)
  (UserInterface|Viewport|AddtoViewport (Variables|Default|GetBossWidget) 0)
  ;[1 1 1] Set physical animation profile for hit reaction
  (Class|PhysicalAnimationComponent|SetSkeletalMeshComponent (Variables|Default|GetPhysicalAnimation) _mesh)
  (Class|SkeletalMeshComponent|SetConstraintProfileforAll _mesh "DamageConstraint" true))

(event Game|Damage|EventAnyDamage
  (params (Damage :type Float%20%28single-precision%29) (DamageType :type Damage%20Type%20Object%20Reference) (InstigatedBy :type Controller%20Object%20Reference) (DamageCauser :type Actor%20Object%20Reference))
  ;[1 1 1] Get damage
  (Utilities|FlowControl|DoOnce false :!label _label
    (:Completed
      (Utilities|FlowControl|Sequence
        (:then_0
          (Variables|Default|Setcurrent_health (- (Variables|Default|Getcurrent_health) Damage))
          (if (<= (Variables|Default|Getcurrent_health) 0.0)
            ;[1 1 1] Death
            (bind _asboss_animation_bluepint (Utilities|Casting|CastToBossAnimationBluepint (Components|SkeletalMesh|GetAnimInstance (Variables|Character|GetMesh))))
            (AI|Logic|StopLogic (Variables|/Script/AIModule.AIController|GetBrainComponent (AI|GetAIController self)) "")
            (Variables|/Game/ExampleBossFightProject/BossAnimationsPack/Animations/BossAnimationBluepint.BossAnimationBluepint_C|SetDeath _asboss_animation_bluepint true)
            (Variables|Default|SetDeath true)
            ;[1 1 1] Remove widget
            (Widget|RemovefromParent (Variables|Default|GetBossWidget))
            ;[1 1 1] Destroy self
            (Utilities|FlowControl|Delay 4.0)
            (Actor|DestroyActor)
            (else
              (Utilities|FlowControl|Delay 0.3)
              (goto _label Reset))))
        (:then_1
          (Class|SkeletalMeshComponent|SetAllBodiesBelowSimulatePhysics (Variables|Character|GetMesh) (Variables|Default|GetBoneName) true true)
          (bind _newtrack_0 (Timeline|PhysicsTimeline PlayFromStart)
            (:Update
              (Variables|Default|SetPhysics%20Blend%20Weight _newtrack_0)
              (Physics|AddImpulse (Variables|Character|GetMesh) "200.000000,200.000000, 0" "spine_01" false))
            (:Finished
              (Class|SkeletalMeshComponent|SetAllBodiesBelowSimulatePhysics (Variables|Character|GetMesh) (Variables|Default|GetBoneName) false true))))
        (:then_2
          ;[1 1 1] Screen shake
          (Timeline|ScreenShakeTimeline PlayFromStart
            (:Update
              (Camera|PlayWorldCameraShake "/Game/ExampleBossFightProject/SwordAnimationPack/screen_shake/BossDamageShake.BossDamageShake_C" (Transformation|GetActorLocation (Game|Player|GetPlayerPawn 0)) 1.5e+02 3e+02))))))))

(event EventTick
  (params (DeltaSeconds :type Float%20%28single-precision%29))
  ;[1 1 1] Turn characters face to the player
  (if (not (Variables|Default|GetDeath))
    (Transformation|SetActorRotation (Math|Rotator|MakeRotator 0.0 0.0 (- (.yaw (Math|Rotator|FindLookatRotation (Transformation|GetActorLocation) (Transformation|GetActorLocation (Game|Player|GetPlayerPawn 0)))) 5.0)))
    (CallFunction|PhysicalHitReact)))

(fn ConstructionScript)